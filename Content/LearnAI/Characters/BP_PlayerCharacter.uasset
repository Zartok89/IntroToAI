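; BP_PlayerCharacter is a player character Blueprint whose camera uses a fixed viewpoint placed in the level instead of following the character.
; On BeginPlay it finds the first CameraActor tagged "CameraView", detaches its FollowCamera component and snaps that camera to the actor's world location and rotation.
; Tick, overlap and construction script are empty.
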(event EventBeginPlay
  (bind _outactors (Actor|GetAllActorsOfClasswithTag "/Script/Engine.CameraActor" "CameraView"))
  (Variables|Default|SetCameraRef (Utilities|Array|Get(acopy) _outactors))
  (Transformation|DetachFromComponent (Variables|Default|GetFollowCamera) "KeepRelative" "KeepRelative" "KeepRelative" true)
  (Transformation|SetWorldLocation (Variables|Default|GetFollowCamera) (Transformation|GetActorLocation (Variables|Default|GetCameraRef)) false false)
  (Transformation|SetWorldRotation (Variables|Default|GetFollowCamera) (Transformation|GetActorRotation (Variables|Default|GetCameraRef)) false false))

(event Collision|EventActorBeginOverlap
  (params (OtherActor :type Actor%20Object%20Reference)))

(event EventTick
  (params (DeltaSeconds :type Float%20%28single-precision%29)))

(fn ConstructionScript)